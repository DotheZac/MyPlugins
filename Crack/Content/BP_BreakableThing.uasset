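; Breakable glass actor that shows spreading cracks, then shatters a Geometry Collection when its IsBreak flag is set.
; The hidden IntactMesh supplies collision while the visible collection stays inert, with ForceBrokenForCustomRenderer enabled.
; Tick steadily raises CrackProgress into custom primitive data and a material parameter, and polls IsBreak.
; BreakGlass runs once, moving collision to the collection, enabling physics, crumbling clusters and applying a radial impulse.
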(event `self.ReceiveBeginPlay`
  (`SceneComponent.SetVisibility` (`self.IntactMesh`) false false)
  (`PrimitiveComponent.SetCollisionEnabled` (`self.IntactMesh`) "QueryAndPhysics")
  (`SceneComponent.SetVisibility` (`self.GeometryCollection`) true false)
  (`PrimitiveComponent.SetCollisionEnabled` (`self.GeometryCollection`) "NoCollision")
  (`PrimitiveComponent.SetEnableGravity` (`self.GeometryCollection`) false)
  (`PrimitiveComponent.SetSimulatePhysics` (`self.GeometryCollection`) false)
  (`GeometryCollectionComponent.ForceBrokenForCustomRenderer` (`self.GeometryCollection`) true))

(event `self.ReceiveTick`
  (params (DeltaSeconds :type "Float (single-precision)"))
  (set `self.CrackProgress` (+ (`self.CrackProgress`) (* DeltaSeconds 0.2)))
  (`|ExecutionSequence`
    (:`then_0`
      (`PrimitiveComponent.SetCustomPrimitiveDataFloat` (`self.GeometryCollection`) 0 (`self.CrackProgress`)))
    (:`then_1`
      (`MeshComponent.SetScalarParameterValueOnMaterials` (`self.GeometryCollection`) "CrackProgress" (`self.CrackProgress`))
      (if (`self.IsBreak`)
        (`self.BreakGlass`)))))

(event `BreakGlass`
  (bind _geometrycollection (`self.GeometryCollection`))
  (`/Engine/EditorBlueprintResources/StandardMacros.DoOnce` false
    (:`Completed`
      (`SceneComponent.SetVisibility` (`self.IntactMesh`) false false)
      (`PrimitiveComponent.SetCollisionEnabled` (`self.IntactMesh`) "NoCollision")
      (`SceneComponent.SetVisibility` (`self.GeometryCollection`) true false)
      (`PrimitiveComponent.SetCollisionEnabled` (`self.GeometryCollection`) "QueryAndPhysics")
      (`PrimitiveComponent.SetEnableGravity` (`self.GeometryCollection`) true)
      (`PrimitiveComponent.SetSimulatePhysics` (`self.GeometryCollection`) true)
      (`GeometryCollectionComponent.CrumbleActiveClusters` (`self.GeometryCollection`))
      (`PrimitiveComponent.AddRadialImpulse` _geometrycollection (`SceneComponent.K2_GetComponentLocation` _geometrycollection) 150.0 100.0 "RIF_Linear" true))))

(fn `UserConstructionScript`)