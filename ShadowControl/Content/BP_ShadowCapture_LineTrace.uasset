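; Blueprint that estimates how shadowed each listed player character is from a referenced light and passes that value to the character's mesh.
; Every Tick it line traces on Visibility from each character against the light's forward vector, turning blocker distance into a 0–1 value, or zero without a hit.
; One ShadowValue, shared across players, is interpolated toward that result, written to Custom Primitive Data index 0 and debug-printed.
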(event `self.ReceiveTick`
  (params (DeltaSeconds :type "Float (single-precision)"))
  (for (_ _array_index) (`self.PlayerIndex`)
    (bind _returnvalue (`GameplayStatics.GetPlayerCharacter` _array_index))
    (if (`KismetSystemLibrary.IsValid` _returnvalue)
      (bind _returnvalue_location (`KismetMathLibrary.BreakTransform` (`self.GetTransform` _returnvalue)))
      (bind (_outhit _returnvalue_2) (`KismetSystemLibrary.LineTraceSingle` _returnvalue_location (+ (* (`self.GetActorForwardVector` (`self.Light`)) (* (`self.TraceLength`) -1.0)) _returnvalue_location) "TraceTypeQuery1"))
      (bind _output_get (set `self.ShadowValue` (`KismetMathLibrary.FInterpTo` (`self.ShadowValue`) (`KismetMathLibrary.SelectFloat` (`KismetMathLibrary.FClamp` (- 1.0 (/ (`.Distance` (`GameplayStatics.BreakHitResult` _outhit)) (`self.TraceLength`)))) 0.0 _returnvalue_2) DeltaSeconds (`self.InterpSpeed`))))
      (`PrimitiveComponent.SetCustomPrimitiveDataFloat` (`Character.Mesh` _returnvalue) 0 _output_get)
      (`KismetSystemLibrary.PrintString` (`KismetStringLibrary.Conv_DoubleToString` (`self.ShadowValue`))))))

(fn `UserConstructionScript`)