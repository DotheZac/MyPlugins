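; BP_SandDust is an actor that places a configurable Niagara sand dust effect in the level.
; On BeginPlay it pushes its settings into the NSSandDust system: speed, spawn box width, spawn rate and particle lifetime.
; The actor's forward vector sets both the effect's rotation parameter and, scaled by DustSpeed, the initial velocity, so the placed orientation steers the dust.
; The construction script is empty, so these values apply only at play.
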(event `self.ReceiveBeginPlay`
  (bind _returnvalue (`self.GetActorForwardVector`))
  (bind _dustspeed (`self.DustSpeed`))
  (`NiagaraComponent.SetNiagaraVariableVec3` (`self.NS_SandDust`) "Rotation" _returnvalue)
  (`NiagaraComponent.SetVariableFloat` (`self.NS_SandDust`) "MoveSpeed" _dustspeed)
  (`NiagaraComponent.SetNiagaraVariableVec3` (`self.NS_SandDust`) "InitVelocity" (* _returnvalue _dustspeed))
  (`NiagaraComponent.SetNiagaraVariableVec3` (`self.NS_SandDust`) "BoxSize" (`KismetMathLibrary.MakeVector` 20.0 (`self.Width`) 20.0))
  (`NiagaraComponent.SetVariableFloat` (`self.NS_SandDust`) "SpawnRate" (`self.SpawnRate`))
  (`NiagaraComponent.SetVariableFloat` (`self.NS_SandDust`) "LifeTime" (`self.LifeTime`)))

(fn `UserConstructionScript`)