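; BP_WallManager flags wall meshes that sit between the player camera and the player character, via a material parameter.
; Each tick it multi-line-traces from camera to character and collects hit mesh components tagged "Wall".
; It caches one dynamic material instance per wall (slot 0) in a map.
; Comparing against the previous frame's walls, it sets the IsOnRay scalar only on walls entering or leaving the ray.
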(event `self.ReceiveTick`
  (params (DeltaSeconds :type "Float (single-precision)"))
  (bind _returnvalue (`GameplayStatics.GetPlayerCharacter` 0))
  (`KismetArrayLibrary.Array_Clear` (`self.CurrentWalls`))
  (if (`KismetSystemLibrary.IsValid` _returnvalue)
    (bind _outhits (`KismetSystemLibrary.LineTraceMulti` (`PlayerCameraManager.GetCameraLocation` (`GameplayStatics.GetPlayerCameraManager` 0)) (`self.K2_GetActorLocation` _returnvalue) "TraceTypeQuery5"))
    (for _array_element _outhits
      (bind (_bblockinghit _binitialoverlap _time _distance _location _impactpoint _normal _impactnormal _physmat _hitactor _hitcomponent) (`GameplayStatics.BreakHitResult` _array_element))
      (if (`ActorComponent.ComponentHasTag` _hitcomponent "Wall")
        (bind _asmesh_component (cast `MeshComponent` _hitcomponent))
        (`KismetArrayLibrary.Array_AddUnique` (`self.CurrentWalls`) _asmesh_component)))
    (for _array_element_2 (`self.CurrentWalls`)
      (if (not (`.ReturnValue` (`BlueprintMapLibrary.Map_Find` (`self.WallMIDMap`) _array_element_2)))
        (bind _returnvalue_2 (`PrimitiveComponent.CreateDynamicMaterialInstance` _array_element_2 0 (`PrimitiveComponent.GetMaterial` _array_element_2 0) "None"))
        (`BlueprintMapLibrary.Map_Add` (`self.WallMIDMap`) _array_element_2 _returnvalue_2)))
    (for _array_element_3 (`self.PreviousWalls`)
      (if (not (`KismetArrayLibrary.Array_Contains` (`self.CurrentWalls`) _array_element_3))
        (bind (_value _returnvalue_3) (`BlueprintMapLibrary.Map_Find` (`self.WallMIDMap`) _array_element_3))
        (if _returnvalue_3
          (`MaterialInstanceDynamic.SetScalarParameterValue` _value "IsOnRay" 0.0))))
    (for _array_element_4 (`self.CurrentWalls`)
      (if (not (`KismetArrayLibrary.Array_Contains` (`self.PreviousWalls`) _array_element_4))
        (bind (_value_2 _returnvalue_4) (`BlueprintMapLibrary.Map_Find` (`self.WallMIDMap`) _array_element_4))
        (if _returnvalue_4
          (`MaterialInstanceDynamic.SetScalarParameterValue` _value_2 "IsOnRay" 1.0))))
    (set `self.PreviousWalls` (`self.CurrentWalls`))))

(fn `UserConstructionScript`)